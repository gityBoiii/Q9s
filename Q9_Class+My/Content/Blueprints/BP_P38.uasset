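; BP_P38 is a P-38 aircraft actor that flies straight ahead while its two propellers spin.
; Each tick it rolls the Left and Right propeller components by the propeller rotation speed and offsets the actor along its local X axis by the move speed.
; Both motions are scaled by delta time, with no input, physics or steering logic.
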(event EventTick
  (params (DeltaSeconds :type Float%20%28single-precision%29))
  ;[1 1 1] Left Rotate
  (Transformation|AddLocalRotation (Variables|Default|GetLeft) (Math|Rotator|MakeRotator (* (Utilities|Time|GetWorldDeltaSeconds) (Variables|Speed|GetPropellerRotationSpeed)) 0.0 0.0) false false)
  ;[1 1 1] Right Rotate
  (Transformation|AddLocalRotation (Variables|Default|GetRight) (Math|Rotator|MakeRotator (* (Utilities|Time|GetWorldDeltaSeconds) (Variables|Speed|GetPropellerRotationSpeed)) 0.0 0.0) false false)
  ;[1 1 1] Move P38
  (Transformation|AddActorLocalOffset (Math|Vector|MakeVector (* (Utilities|Time|GetWorldDeltaSeconds) (Variables|Speed|GetMoveSpeed)) 0.0 0.0) false false))

(fn ConstructionScript)