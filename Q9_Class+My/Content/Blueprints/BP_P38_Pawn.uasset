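; BP_P38_Pawn is a player-flown P-38 plane pawn that constantly flies forward, steers, boosts and fires rockets.
; Tick spins the Left and Right propellers and feeds forward movement input to the FloatingPawnMovement component.
; Pitch and Roll axes rotate the actor locally, scaled by rotation speed and delta time.
; Boost toggles the movement's max speed while held, and Fire spawns a BP_Rocket at the Arrow component's transform.
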(event EventTick
  (params (DeltaSeconds :type Float%20%28single-precision%29))
  ;[1 1 1] Left Rotate
  (Transformation|AddLocalRotation (Variables|Default|GetLeft) (Math|Rotator|MakeRotator (* (Utilities|Time|GetWorldDeltaSeconds) (Variables|Speed|GetPropellerRotationSpeed)) 0.0 0.0) false false)
  ;[1 1 1] Right Rotate
  (Transformation|AddLocalRotation (Variables|Default|GetRight) (Math|Rotator|MakeRotator (* (Utilities|Time|GetWorldDeltaSeconds) (Variables|Speed|GetPropellerRotationSpeed)) 0.0 0.0) false false)
  ;[1 1 1] FloatingPawn Movment
  (Pawn|Input|AddMovementInput (Transformation|GetActorForwardVector) 1.0 false))

(event Input|ActionEvents|InputActionBoost
  (params (Key :type Key%20Structure :default "None"))
  ;[1 1 1] Boost
  (:Pressed
    (bind _output_get (Variables|Speed|SetMoveSpeed 4e+02))
    (Variables|/Script/Engine.FloatingPawnMovement|SetMaxSpeed (Variables|Default|GetFloatingPawnMovement) _output_get))
  (:Released
    (bind _output_get_2 (Variables|Speed|SetMoveSpeed 5e+01))
    (Variables|/Script/Engine.FloatingPawnMovement|SetMaxSpeed (Variables|Default|GetFloatingPawnMovement) _output_get_2)))

(event Input|ActionEvents|InputActionFire
  (params (Key :type Key%20Structure :default "None"))
  (:Pressed
    (Game|SpawnActorfromClass "/Game/Blueprints/BP_Rocket.BP_Rocket_C" (Transformation|GetWorldTransform (Variables|Default|GetArrow)) "Undefined" 0 0)))

(event Input|AxisEvents|InputAxisPitch
  (params (AxisValue :type Float%20%28single-precision%29))
  ;[1 1 1] Pitch
  (Transformation|AddActorLocalRotation (Math|Rotator|MakeRotator 0.0 (* (Math|Float|Clamp(Float) AxisValue -1.0) (Variables|Speed|GetRoationSpeed) (Utilities|Time|GetWorldDeltaSeconds)) 0.0) false false))

(event Input|AxisEvents|InputAxisRoll
  (params (AxisValue :type Float%20%28single-precision%29))
  ;[1 1 1] Roll
  (Transformation|AddActorLocalRotation (Math|Rotator|MakeRotator (* (Math|Float|Clamp(Float) AxisValue -1.0) (Variables|Speed|GetRoationSpeed) (Utilities|Time|GetWorldDeltaSeconds)) 0.0 0.0) false false))

(fn ConstructionScript)